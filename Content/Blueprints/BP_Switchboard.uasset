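; Switchboard pawn that a player possesses through a hold interaction to repair BP_Light actors in its editable region with F6.
; Interacting shows the mouse, swings the door open through RPS-to-RPC replication events and lerps the camera from the player's view to the board's.
; Pause returns possession to the player and shuts the door.
; It also supplies interaction prompts, including an in-use message, and a turbulence camera shake.
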(event `self.ReceiveBeginPlay`
  ;[0.05098 0.05098 0.05098] Set target camera transform
  (set `self.TargetCameraTransform` (`SceneComponent.K2_GetComponentToWorld` (`self.Camera`))))

(event `/Game/Blueprints/Interfaces/BPI_Interaction.GetText`
  (params (PlayerRef :type "/Game/Blueprints/BP_PlayerCharacter Object Reference") (ObjectType :type "ECollisionChannel Enum" :default "ECC_WorldStatic"))
  (bind _playerref (`self.PlayerRef`))
  ;[0.05098 0.05098 0.05098] Send text to player widget
  (set `self.PlayerRef` PlayerRef)
  (bind _output_get (set `self.ObjectType` ObjectType))
  (switch `ECollisionChannel` _output_get
    (:`ECC_GameTraceChannel2`
      (message `/Game/Blueprints/Interfaces/BPI_PlayerCharacter.RecieveText` _playerref "E" "Access switchboard"))
    (:`ECC_GameTraceChannel3`
      (message `/Game/Blueprints/Interfaces/BPI_PlayerCharacter.RecieveText` _playerref "" "Someone is already using this"))))

(event `Key|F6`
  (params (Key :type "Key Structure"))
  ;[1 0 0] Repair lights (only server can do)
  (:`Pressed`
    (for _array_element (`PrimitiveComponent.GetOverlappingActors` (`self.FixTheseLights`) "/Game/Blueprints/BP_Light.BP_Light_C")
      (message `/Game/Blueprints/Interfaces/BPI_Environment.Repair` _array_element))))

(event `/Game/Blueprints/Interfaces/BPI_Interaction.Interact`
  (params (ControllerRef :type "Controller Object Reference"))
  (switch `ECollisionChannel` (`self.ObjectType`)
    (:`ECC_GameTraceChannel2`
      (bind _output_get (set `self.ControllerRef` ControllerRef))
      (bind _output_get_2 (set `self.RePossessionPlayerRef` (`self.PlayerRef`)))
      (message `/Game/Blueprints/Interfaces/BPI_PlayerCharacter.PossessTarget` _output_get_2 self _output_get true)
      (`self.OpenDoor`)
      (`self.FocusCamera`))))

(event `RPS_ToggleDoor`
  (params (Z :type "Float (single-precision)"))
  ;[0.05098 0.05098 0.05098] Toggle door
  (`self.RPC_ToggleDoor` Z))

(event `RPC_ToggleDoor`
  (params (Z :type "Float (single-precision)"))
  ;[0.05098 0.05098 0.05098] Toggle door
  (`SceneComponent.K2_SetRelativeRotation` (`self.Door`) (`KismetMathLibrary.MakeRotator` 0.0 0.0 Z) false false))

(event `OpenDoor`
  ;[0.05098 0.05098 0.05098] Toggle door
  (bind (_direction _z) (`Timeline|ToggleDoor` :!via `PlayFromStart` :!label _label)
    (:`Update`
      (`self.RPS_ToggleDoor` _z))))

(event `ShutDoor`
  ;[0.05098 0.05098 0.05098] Toggle door
  (goto _label :!via `ReverseFromEnd`))

(event `FocusCamera`
  ;[0.05098 0.05098 0.05098] Focus camera when possessed
  (set `self.PreviousCameraTransform` (`SceneComponent.K2_GetComponentToWorld` (`/Game/Blueprints/BP_PlayerCharacter.Camera` (`self.PlayerRef`))))
  (bind (_direction _lerpalpha) (`Timeline|LerpCamera` :!via `PlayFromStart`)
    (:`Update`
      (`SceneComponent.K2_SetWorldTransform` (`self.Camera`) (`KismetMathLibrary.TLerp` (`self.PreviousCameraTransform`) (`self.TargetCameraTransform`) _lerpalpha) false false))))

(event `EnhancedInput|/Game/Blueprints/Inputs/IA_Pause`
  (params (ActionValue :type Boolean) (ElapsedSeconds :type "Float (double-precision)") (TriggeredSeconds :type "Float (double-precision)") (InputAction :type "InputAction Object Reference" :default "/Game/Blueprints/Inputs/IA_Pause.IA_Pause"))
  (:`Started`
    (`self.RPS_UnPossess` (`self.ControllerRef`) (`self.RePossessionPlayerRef`))))

(event `RPS_UnPossess`
  (params (ControllerRef :type "Controller Object Reference") (PlayerRef :type "/Game/Blueprints/BP_PlayerCharacter Object Reference"))
  (`Controller.Possess` ControllerRef PlayerRef)
  (`self.ShutDoor`))

(event `RPC_Turbulence`
  (`GameplayStatics.PlayWorldCameraShake` "/Game/Blueprints/CameraShake/BP_CameraShakeTurbulence.BP_CameraShakeTurbulence_C" (`self.K2_GetActorLocation`) 0.0 250.0))

(fn `UserConstructionScript`
  (`SceneComponent.K2_SetRelativeTransform` (`self.FixTheseLights`) (`self.AffectedRegion`) false false))