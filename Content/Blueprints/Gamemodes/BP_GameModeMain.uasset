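; Main game mode that tracks connected players, spawns their characters and triggers basic moth enemy waves.
; Login, seamless controller swap and logout events maintain the player list.
; SpawnPlayer replaces a controller's pawn with a new BP_PlayerCharacter at the first untaken PlayerStart, then tags that start "Taken".
; CheckEnemyLeft calls for a moth wave respawn when no enemies are alive, first running one tick after BeginPlay.
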(event `self.K2_PostLogin`
  (params (NewPlayer :type "PlayerController Object Reference"))
  ;[1 1 1] Managing Player List
  (`KismetArrayLibrary.Array_Add` (`self.PlayerList`) NewPlayer))

(event `self.K2_OnSwapPlayerControllers`
  (params (OldPC :type "PlayerController Object Reference") (NewPC :type "PlayerController Object Reference"))
  ;[1 1 1] Managing Player List
  (`KismetArrayLibrary.Array_Add` (`self.PlayerList`) NewPC))

(event `self.K2_OnLogout`
  (params (ExitingController :type "Controller Object Reference"))
  ;[1 1 1] Managing Player List
  (bind _asplayer_controller (cast `PlayerController` ExitingController))
  (`KismetArrayLibrary.Array_RemoveItem` (`self.PlayerList`) _asplayer_controller))

(event `CheckEnemyLeft`
  (if (== (`self.EnemyAlive`) 0)
    (`self.RespawnBasicMothWave`)))

(event `self.ReceiveBeginPlay`
  (`KismetSystemLibrary.DelayUntilNextTick`)
  (`self.CheckEnemyLeft`))

(fn `ChoosePlayerStart`
  (params (Player :type "Controller Object Reference"))
  (returns (ReturnValue :type "Actor Object Reference"))
  (return Player))

(fn `FindAvailablePlayerStart`
  (returns (PlayerStartTransorm :type "Transform Structure (by ref)") (PlayerStartRef :type "PlayerStart Object Reference"))
  ;[0.05098 0.05098 0.05098] Find available player start
  (bind _outactors (`GameplayStatics.GetAllActorsOfClass` "/Script/Engine.PlayerStart"))
  (for _array_element _outactors
    (if (!= (`PlayerStart.PlayerStartTag` _array_element) "Taken")
      (return (`self.GetTransform` _array_element) _array_element))))

(fn `SpawnPlayer`
  (params (PlayerController :type "PlayerController Object Reference"))
  (bind _returnvalue (`Controller.K2_GetPawn` PlayerController))
  (bind (_playerstarttransorm _playerstartref) (`self.FindAvailablePlayerStart`))
  ;[0.05098 0.05098 0.05098] Spawn player
  (`/Engine/EditorBlueprintResources/StandardMacros.IsValid` _returnvalue
    (:`Is Valid`
      (`self.K2_DestroyActor` _returnvalue))
    (:`Is Not Valid`
      _))
  (bind _returnvalue_2 (`|SpawnActorFromClass` "/Game/Blueprints/BP_PlayerCharacter.BP_PlayerCharacter_C" _playerstarttransorm "Undefined" "MultiplyWithRoot" null null))
  (`Controller.Possess` PlayerController _returnvalue_2)
  (set `PlayerStart.PlayerStartTag` "Taken" _playerstartref))

(fn `UserConstructionScript`)