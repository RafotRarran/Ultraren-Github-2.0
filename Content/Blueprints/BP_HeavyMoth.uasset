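; BP_HeavyMoth is an enemy that runs the heavy flying AI behavior tree and counts toward the game mode's living enemy total.
; On BeginPlay, the authority starts the tree on its AI controller and increments EnemyAlive in BP_GameModeMain.
; AnyDamage reduces clamped health; at zero it decrements that count, has the game mode check remaining enemies and destroys the actor, otherwise printing a debug message.
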(event `self.ReceiveBeginPlay`
  (if (`self.HasAuthority`)
    (`AIController.RunBehaviorTree` (`AIBlueprintHelperLibrary.GetAIController` self) "/Game/Blueprints/AI/BT_HeavyFlyingAI1.BT_HeavyFlyingAI1")
    (bind _asbp_game_mode_main (cast `/Game/Blueprints/Gamemodes/BP_GameModeMain` (`GameplayStatics.GetGameMode`)))
    (`/Engine/EditorBlueprintResources/StandardMacros.IncrementInt` (`/Game/Blueprints/Gamemodes/BP_GameModeMain.EnemyAlive` _asbp_game_mode_main))))

(event `self.ReceiveAnyDamage`
  (params (Damage :type "Float (single-precision)") (DamageType :type "DamageType Object Reference") (InstigatedBy :type "Controller Object Reference") (DamageCauser :type "Actor Object Reference"))
  (bind _output_get (set `self.CurrentHealth` (`KismetMathLibrary.FClamp` (- (`self.CurrentHealth`) Damage) 0.0 100.0)))
  (if (== _output_get 0.0)
    (bind _asbp_game_mode_main (cast `/Game/Blueprints/Gamemodes/BP_GameModeMain` (`GameplayStatics.GetGameMode`)))
    (`/Engine/EditorBlueprintResources/StandardMacros.DecrementInt` (`/Game/Blueprints/Gamemodes/BP_GameModeMain.EnemyAlive` _asbp_game_mode_main)
      (:`  `
        (`/Game/Blueprints/Gamemodes/BP_GameModeMain.CheckEnemyLeft` _asbp_game_mode_main)
        (`self.K2_DestroyActor`)))
    (else
      (`KismetSystemLibrary.PrintString` "Damaged"))))

(fn `UserConstructionScript`)