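; BP_EnvironmentManager broadcasts a turbulence effect to affected actors in the level through a single Turbulence event.
; The event runs a Sequence that finds every light, player character, turret and switchboard with GetAllActorsOfClass at call time.
; Lights receive a Flicker call, while the other three classes each receive their own RPCTurbulence call, leaving each response to the receiving Blueprint.
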(event `Turbulence`
  (`|ExecutionSequence`
    (:`then_0`
      (bind _outactors (`GameplayStatics.GetAllActorsOfClass` "/Game/Blueprints/BP_Light.BP_Light_C"))
      (for _array_element _outactors
        (`/Game/Blueprints/BP_Light.Flicker` _array_element)))
    (:`then_1`
      (bind _outactors_2 (`GameplayStatics.GetAllActorsOfClass` "/Game/Blueprints/BP_PlayerCharacter.BP_PlayerCharacter_C"))
      (for _array_element_2 _outactors_2
        (`/Game/Blueprints/BP_PlayerCharacter.RPC_Turbulence` _array_element_2)))
    (:`then_2`
      (bind _outactors_3 (`GameplayStatics.GetAllActorsOfClass` "/Game/Blueprints/BP_Turret.BP_Turret_C"))
      (for _array_element_3 _outactors_3
        (`/Game/Blueprints/BP_Turret.RPC_Turbulence` _array_element_3)))
    (:`then_3`
      (bind _outactors_4 (`GameplayStatics.GetAllActorsOfClass` "/Game/Blueprints/BP_Switchboard.BP_Switchboard_C"))
      (for _array_element_4 _outactors_4
        (`/Game/Blueprints/BP_Switchboard.RPC_Turbulence` _array_element_4)))))

(fn `UserConstructionScript`)