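; BP_BasicMoth is a flying enemy that lives for a limited time and counts toward the game mode's enemy total.
; On BeginPlay, the server starts BT_BasicFlyingAI on its AI controller and increments EnemyAlive in BP_GameModeMain.
; After a fixed delay, it decrements that count, calls CheckEnemyLeft and destroys itself.
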(event `self.ReceiveBeginPlay`
  (if (`self.HasAuthority`)
    (`AIController.RunBehaviorTree` (`AIBlueprintHelperLibrary.GetAIController` self) "/Game/Blueprints/AI/BT_BasicFlyingAI.BT_BasicFlyingAI")
    (bind _asbp_game_mode_main (cast `/Game/Blueprints/Gamemodes/BP_GameModeMain` (`GameplayStatics.GetGameMode`)))
    (`/Engine/EditorBlueprintResources/StandardMacros.IncrementInt` (`/Game/Blueprints/Gamemodes/BP_GameModeMain.EnemyAlive` _asbp_game_mode_main)
      (:`  `
        (`KismetSystemLibrary.Delay` 200.0)
        (bind _asbp_game_mode_main_2 (cast `/Game/Blueprints/Gamemodes/BP_GameModeMain` (`GameplayStatics.GetGameMode`)))
        (`/Engine/EditorBlueprintResources/StandardMacros.DecrementInt` (`/Game/Blueprints/Gamemodes/BP_GameModeMain.EnemyAlive` _asbp_game_mode_main_2)
          (:`  `
            (`/Game/Blueprints/Gamemodes/BP_GameModeMain.CheckEnemyLeft` _asbp_game_mode_main_2)
            (`self.K2_DestroyActor`)))))))

(fn `UserConstructionScript`)