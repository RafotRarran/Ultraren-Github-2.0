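; Behavior tree task that makes a BP_BasicMoth spit acid at the blackboard TargetLocation.
; When the target is within SpitRange of the moth's Mouth, a line trace checks that the first hit actor is tagged Destructible.
; If so, it spawns BP_AcidSpit at the mouth, rotated toward the target through RInterpTo.
; The task finishes successfully whether or not it fires, provided the pawn cast succeeds.
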(event `self.ReceiveExecuteAI`
  (params (OwnerController :type "AIController Object Reference") (ControlledPawn :type "Pawn Object Reference"))
  (bind _returnvalue (`BTFunctionLibrary.GetBlackboardValueAsVector` (`self.TargetLocation`)))
  (bind _asbp_basic_moth (cast `/Game/Blueprints/BP_BasicMoth` ControlledPawn))
  (bind _mouth (`/Game/Blueprints/BP_BasicMoth.Mouth` _asbp_basic_moth))
  (bind _returnvalue_location (`KismetMathLibrary.BreakTransform` (`SceneComponent.K2_GetComponentToWorld` _mouth)))
  (if (== _returnvalue_location _returnvalue :`ErrorTolerance` (`self.SpitRange`))
    (bind _outhit (`KismetSystemLibrary.LineTraceSingleByProfile` _returnvalue_location _returnvalue))
    (`/Engine/EditorBlueprintResources/StandardMacros.IsValid` (`.HitActor` (`GameplayStatics.BreakHitResult` _outhit))
      (:`Is Valid`
        (if (`Actor.ActorHasTag` (`.HitActor` (`GameplayStatics.BreakHitResult` _outhit)) "Destructible")
          (`|SpawnActorFromClass` "/Game/Blueprints/BP_AcidSpit.BP_AcidSpit_C" (`KismetMathLibrary.MakeTransform` _returnvalue_location (`KismetMathLibrary.RInterpTo` (`SceneComponent.K2_GetComponentRotation` _mouth) (`KismetMathLibrary.FindLookAtRotation` (`SceneComponent.K2_GetComponentLocation` _mouth) _returnvalue) (`GameplayStatics.GetWorldDeltaSeconds`))) "AlwaysSpawn" "MultiplyWithRoot" null null)
          (`self.FinishExecute` true)
          (else
            (`self.FinishExecute` true))))
      (:`Is Not Valid`
        (`self.FinishExecute` true)))
    (else
      (`self.FinishExecute` true))))