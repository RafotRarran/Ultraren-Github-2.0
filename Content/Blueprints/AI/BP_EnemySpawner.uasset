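; Enemy spawner that spawns waves of heavy moths when the main game mode signals a wave respawn.
; On BeginPlay it binds SpawnEnemy to BP_GameModeMain's basic moth wave respawn event, despite that event's name.
; Each wave spawns EnemySpawned heavy moths near randomly picked HeavySpawns points, then increments the count.
; A basic moth function using random circumference points and heights exists but is not called here.
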(event `self.ReceiveBeginPlay`
  (bind _asbp_game_mode_main (cast `/Game/Blueprints/Gamemodes/BP_GameModeMain` (`GameplayStatics.GetGameMode`)))
  (add `/Game/Blueprints/Gamemodes/BP_GameModeMain.RespawnBasicMothWave` _asbp_game_mode_main (delegate `SpawnEnemy`)))

(event `SpawnEnemy`
  (for _ (range (`self.EnemySpawned`))
    (`self.FNC_SpawnHeavyMoth`))
  (`/Engine/EditorBlueprintResources/StandardMacros.IncrementInt` (`self.EnemySpawned`)))

(fn `FNC_FindPointOnCircumference`
  (bind _radius (`self.Radius`))
  (set `self.Degrees` (`KismetMathLibrary.RandomFloatInRange` 0.0 360.0))
  (set `self.SpawnPointX` (* _radius (`KismetMathLibrary.DegCos` (`self.Degrees`))))
  (set `self.SpawnPointY` (* (`KismetMathLibrary.DegSin` (`self.Degrees`)) _radius)))

(fn `FNC_SpawnBasicMoth`
  (`self.FNC_FindPointOnCircumference`)
  (`|SpawnActorFromClass` "/Game/Blueprints/BP_BasicMoth.BP_BasicMoth_C" (`KismetMathLibrary.MakeTransform` (`KismetMathLibrary.MakeVector` (`self.SpawnPointX`) (`self.SpawnPointY`) (`KismetMathLibrary.RandomFloatInRange` 900.0 1200.0))) "AdjustIfPossibleButAlwaysSpawn" "MultiplyWithRoot" null null))

(fn `FNC_SpawnHeavyMoth`
  (`|SpawnActorFromClass` "/Game/Blueprints/BP_HeavyMoth.BP_HeavyMoth_C" (`KismetMathLibrary.Conv_VectorToTransform` (`KismetMathLibrary.RandomPointInBoundingBox` (`KismetArrayLibrary.Array_Random` (`self.HeavySpawns`)) (50.0 50.0 50.0))) "AlwaysSpawn" "MultiplyWithRoot" null null))

(fn `UserConstructionScript`)