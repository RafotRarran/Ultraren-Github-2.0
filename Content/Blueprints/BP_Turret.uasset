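; Mountable turret pawn that players use via an interaction prompt, possess to aim and fire, and leave with the pause input.
; RPS-to-RPC event pairs relay possession, rotation and exit, restoring the player's camera, collision and interaction on exit.
; Look input is speed-clamped, turning the base by yaw and the guns by pitch.
; Firing runs a delay timeline, then two randomly spread, debug-drawn line traces from the barrel arrows, without applying damage.
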(event `RPS_EventPossessed`
  (params (ControllerRef :type "Controller Object Reference") (RestingRotation :type "Rotator Structure"))
  ;[0.05098 0.05098 0.05098] Setup pawn properties upon possession
  (`self.RPC_EventPossessed` ControllerRef RestingRotation))

(event `RPC_EventPossessed`
  (params (ControllerRef :type "Controller Object Reference") (RestingRotation :type "Rotator Structure"))
  (bind _returnvalue (`GameplayStatics.GetPlayerCameraManager` 0))
  (bind _playerref (`self.PlayerRef`))
  (bind (_returnvalue_roll _returnvalue_pitch _returnvalue_yaw) (`KismetMathLibrary.BreakRotator` (`SceneComponent.K2_GetComponentRotation` (`self.Camera`))))
  ;[0.05098 0.05098 0.05098] Setup pawn properties upon possession
  (`Controller.SetControlRotation` ControllerRef RestingRotation)
  (`/Engine/EditorBlueprintResources/StandardMacros.IsValid` _playerref
    (:`Is Valid`
      (if (`/Game/Blueprints/BP_PlayerCharacter.MainWidgetReady` _playerref)
        (`Widget.SetVisibility` (`/Game/Blueprints/BP_PlayerCharacter.MainWidgetRef` _playerref) "Hidden")
        (set `PlayerCameraManager.ViewPitchMin` -7.5 _returnvalue)
        (set `PlayerCameraManager.ViewPitchMax` 82.5 _returnvalue)
        (`SceneComponent.K2_SetWorldRotation` (`self.TurretBase`) (`KismetMathLibrary.MakeRotator` _returnvalue_roll _returnvalue_pitch (- _returnvalue_yaw 90.0)) false false)))))

(event `self.ReceivePossessed`
  (params (NewController :type "Controller Object Reference"))
  ;[0.05098 0.05098 0.05098] Setup pawn properties upon possession
  (`/Engine/EditorBlueprintResources/StandardMacros.IsValid` NewController
    (:`Is Valid`
      (bind _output_get (set `self.ControllerRef` NewController))
      (`self.RPS_EventPossessed` _output_get (`self.RestingRotation`)))))

(event `/Game/Blueprints/Interfaces/BPI_Interaction.GetText`
  (params (PlayerRef :type "/Game/Blueprints/BP_PlayerCharacter Object Reference") (ObjectType :type "ECollisionChannel Enum" :default "ECC_WorldStatic"))
  (bind _playerref (`self.PlayerRef`))
  ;[0.05098 0.05098 0.05098] Send text to player widget
  (set `self.PlayerRef` PlayerRef)
  (bind _output_get (set `self.ObjectTypeRef` ObjectType))
  (switch `ECollisionChannel` _output_get
    (:`ECC_GameTraceChannel1`
      (message `/Game/Blueprints/Interfaces/BPI_PlayerCharacter.RecieveText` _playerref "E" "Reload turret"))
    (:`ECC_GameTraceChannel2`
      (message `/Game/Blueprints/Interfaces/BPI_PlayerCharacter.RecieveText` _playerref "E" "Use turret"))
    (:`ECC_GameTraceChannel3`
      (message `/Game/Blueprints/Interfaces/BPI_PlayerCharacter.RecieveText` _playerref "" "This turret is already in use"))))

(event `/Game/Blueprints/Interfaces/BPI_Interaction.Interact`
  (params (ControllerRef :type "Controller Object Reference"))
  ;[0.05098 0.05098 0.05098] Handle interaction
  (if (not (`self.Possessed`))
    (set `self.ControllerRef` ControllerRef)
    (switch `ECollisionChannel` (`self.ObjectTypeRef`)
      (:`ECC_GameTraceChannel2`
        (message `/Game/Blueprints/Interfaces/BPI_PlayerCharacter.PossessTurret` (`self.PlayerRef`) self (`self.ControllerRef`))))))

(event `RPS_Rotate`
  (params (Pitch :type "Float (double-precision)") (Yaw :type "Float (double-precision)"))
  ;[1 1 1] Limit turning speed and match static mesh rotation with camera rotation
  (`self.RPC_Rotate` Pitch Yaw))

(event `EnhancedInput|/Game/Blueprints/Inputs/Movement/IA_Look`
  (params (ActionValue :type "Vector2D Structure") (ElapsedSeconds :type "Float (double-precision)") (TriggeredSeconds :type "Float (double-precision)") (InputAction :type "InputAction Object Reference" :default "/Game/Blueprints/Inputs/Movement/IA_Look.IA_Look"))
  (bind _turningspeedclamp (`self.TurningSpeedClamp`))
  (bind (_returnvalue_roll _returnvalue_pitch _returnvalue_yaw) (`KismetMathLibrary.BreakRotator` (`SceneComponent.K2_GetComponentRotation` (`self.Camera`))))
  (bind _returnvalue (* _turningspeedclamp -1.0))
  ;[1 1 1] Limit turning speed and match static mesh rotation with camera rotation
  (:`Triggered`
    (`self.AddControllerYawInput` (`KismetMathLibrary.FClamp` ActionValue_X _returnvalue _turningspeedclamp))
    (`self.AddControllerPitchInput` (`KismetMathLibrary.FClamp` ActionValue_Y _returnvalue _turningspeedclamp))
    (`self.RPS_Rotate` (* _returnvalue_pitch -1.0) (- _returnvalue_yaw 90.0))))

(event `EnhancedInput|/Game/Blueprints/Inputs/IA_Pause`
  (params (ActionValue :type Boolean) (ElapsedSeconds :type "Float (double-precision)") (TriggeredSeconds :type "Float (double-precision)") (InputAction :type "InputAction Object Reference" :default "/Game/Blueprints/Inputs/IA_Pause.IA_Pause"))
  ;[1 1 1] Unpossess turret
  (:`Triggered`
    (`self.RPS_UnPossessTurret` (`self.ControllerRef`) (`self.PlayerRef`))))

(event `RPC_Rotate`
  (params (Pitch :type "Float (double-precision)") (Yaw :type "Float (double-precision)"))
  (bind _turretguns (`self.TurretGuns`))
  (bind _turretbase (`self.TurretBase`))
  (bind (_returnvalue_roll _returnvalue_pitch _returnvalue_yaw) (`KismetMathLibrary.BreakRotator` (`SceneComponent.K2_GetComponentRotation` _turretguns)))
  (bind (_returnvalue_roll_2 _returnvalue_pitch_2) (`KismetMathLibrary.BreakRotator` (`SceneComponent.K2_GetComponentRotation` _turretbase)))
  ;[1 1 1] Limit turning speed and match static mesh rotation with camera rotation
  (`SceneComponent.K2_SetWorldRotation` _turretbase (`KismetMathLibrary.MakeRotator` _returnvalue_roll_2 _returnvalue_pitch_2 Yaw) false false)
  (`SceneComponent.K2_SetWorldRotation` _turretguns (`KismetMathLibrary.MakeRotator` Pitch _returnvalue_pitch _returnvalue_yaw) false false))

(event `RPS_UnPossessTurret`
  (params (ControllerRef :type "Controller Object Reference") (PlayerRef :type "/Game/Blueprints/BP_PlayerCharacter Object Reference"))
  ;[1 1 1] Unpossess turret
  (`Controller.Possess` ControllerRef PlayerRef)
  (`self.RPC_UnPossessTurret` PlayerRef))

(event `RPC_UnPossessTurret`
  (params (PlayerRef :type "/Game/Blueprints/BP_PlayerCharacter Object Reference"))
  ;[1 1 1] Unpossess turret
  (set `self.Possessed` false)
  (`PrimitiveComponent.SetCollisionObjectType` (`self.UseTurretCollider`) "ECC_GameTraceChannel2")
  (`/Game/Blueprints/BP_PlayerCharacter.OpenInteractionGate` PlayerRef)
  (`SceneComponent.SetVisibility` (`/Game/Blueprints/BP_PlayerCharacter.Camera` PlayerRef) true true)
  (`self.SetActorEnableCollision` PlayerRef true))

(event `EnhancedInput|/Game/Blueprints/Inputs/IA_Primary`
  (params (ActionValue :type Boolean) (ElapsedSeconds :type "Float (double-precision)") (TriggeredSeconds :type "Float (double-precision)") (InputAction :type "InputAction Object Reference" :default "/Game/Blueprints/Inputs/IA_Primary.IA_Primary"))
  ;[1 1 1] Fire
  (:`Triggered`
    (`self.RPS_Fire`)))

(event `RPS_Fire`
  (bind _leftarrow (`self.LeftArrow`))
  (bind _rightarrow (`self.RightArrow`))
  (bind (_returnvalue_x _returnvalue_y _returnvalue_z) (`KismetMathLibrary.BreakVector` (`SceneComponent.GetForwardVector` _leftarrow)))
  (bind _returnvalue (`SceneComponent.K2_GetComponentLocation` _leftarrow))
  (bind _returnvalue_2 (`SceneComponent.K2_GetComponentLocation` _rightarrow))
  (bind (_returnvalue_x_2 _returnvalue_y_2 _returnvalue_z_2) (`KismetMathLibrary.BreakVector` (`SceneComponent.GetForwardVector` _rightarrow)))
  ;[1 1 1] Fire
  (`Timeline|FiringDelay` :!label _label
    (:`Finished`
      (`|ExecutionSequence`
        (:`then_0`
          (`KismetSystemLibrary.PrintString` "Dvv")
          (`KismetSystemLibrary.LineTraceSingle` :`Start` _returnvalue :`End` (+ _returnvalue (* (`KismetMathLibrary.MakeVector` (+ _returnvalue_x (`KismetMathLibrary.RandomFloatInRange` -0.02 0.02)) _returnvalue_y (+ _returnvalue_z (`KismetMathLibrary.RandomFloatInRange` -0.02 0.02))) 2500.0)) :`TraceChannel` "TraceTypeQuery1" :`DrawDebugType` "ForDuration")
          (`KismetSystemLibrary.LineTraceSingle` :`Start` _returnvalue_2 :`End` (+ _returnvalue_2 (* (`KismetMathLibrary.MakeVector` (+ _returnvalue_x_2 (`KismetMathLibrary.RandomFloatInRange` -0.02 0.02)) _returnvalue_y_2 (+ _returnvalue_z_2 (`KismetMathLibrary.RandomFloatInRange` -0.02 0.02))) 2500.0)) :`TraceChannel` "TraceTypeQuery1" :`DrawDebugType` "ForDuration"))
        (:`then_1`
          (goto _label :!via `SetNewTime`))))))

(fn `UserConstructionScript`
  (set `self.RestingRotation` (`self.K2_GetActorRotation`)))