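; BP_Light is a lamp that can be switched on and off and can flicker during turbulence.
; TurnOn and TurnOff toggle the spotlight's visibility and swap the lamp's bulb material.
; RPS events relay to RPC events that call these functions, a layering whose names suggest server-to-client replication.
; Turbulence has a coin-flip chance to run a delayed loop of randomly timed off/on flickers through the RPS events.
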(event `RPS_TurnOff`
  (`self.RPC_TurnOff`))

(event `RPC_TurnOff`
  (`self.TurnOff`))

(event `TurnOff`
  (`SceneComponent.SetVisibility` (`self.SpotLight`) false true)
  (`PrimitiveComponent.SetMaterial` (`self.Lamp`) 0 "/Game/Materials/Light/M_LightBulbOff.M_LightBulbOff"))

(event `RPS_TurnOn`
  (`self.RPC_TurnOn`))

(event `RPC_TurnOn`
  (`self.TurnOn`))

(event `TurnOn`
  (`SceneComponent.SetVisibility` (`self.SpotLight`) true true)
  (`PrimitiveComponent.SetMaterial` (`self.Lamp`) 0 "/Game/Materials/Light/M_LightBulb.M_LightBulb"))

(event `Turbulence`
  (if (== (`KismetMathLibrary.RandomIntegerInRange` 1 2) 1)
    (`/Game/Blueprints/BP_MacroLibrary.ForLoopWithDelay` 1 (`KismetMathLibrary.RandomIntegerInRange` 3 6) (`KismetMathLibrary.RandomFloatInRange` 0.5 0.8)
      (:`Then`
        (`self.RPS_TurnOff`)
        (`KismetSystemLibrary.Delay` (`KismetMathLibrary.RandomFloatInRange` 0.1 0.4))
        (`self.RPS_TurnOn`)))))

(fn `UserConstructionScript`)