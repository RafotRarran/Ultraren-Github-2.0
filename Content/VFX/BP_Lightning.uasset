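; BP_Lightning is a lightning effect that strikes on an endless loop at random intervals, starting at BeginPlay.
; Each strike plays the Thunder_Strike timeline, driving the Y and Emission material parameters on ThunderPlane.
; Shortly after the strike begins, the loop briefly raises manual exposure compensation on PPVolume to flash the scene.
; It then restores a hard-coded base exposure rather than the volume's original setting.
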(event `self.ReceiveBeginPlay`
  (bind _pp_volume (`self.PP_Volume`))
  (`KismetSystemLibrary.Delay` (`KismetMathLibrary.RandomFloatInRange` 1.0 60.0) :!label _label)
  (`self.Strike`)
  (`KismetSystemLibrary.Delay` 0.2)
  (bind _output_get (set `self.Original Exposure Compensation` 11.0))
  (set `PostProcessVolume.Settings` (make `PostProcessSettings` :`AutoExposureMethod` "AEM_Manual" :`AutoExposureBias` 12.0) _pp_volume)
  (`KismetSystemLibrary.Delay` 0.2)
  (set `PostProcessVolume.Settings` (make `PostProcessSettings` :`AutoExposureMethod` "AEM_Manual" :`AutoExposureBias` _output_get) _pp_volume)
  (goto _label))

(event `Strike`
  (bind _thunder_plane (`self.Thunder_Plane`))
  (bind (_direction _y) (`Timeline|Thunder_Strike` :!via `PlayFromStart`)
    (:`Update`
      (`MeshComponent.SetScalarParameterValueOnMaterials` _thunder_plane "Y" _y)
      (`MeshComponent.SetScalarParameterValueOnMaterials` _thunder_plane "Emission" (* (+ _y 1.0) 1000.0)))))

(fn `UserConstructionScript`)